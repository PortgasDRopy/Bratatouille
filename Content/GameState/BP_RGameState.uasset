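; Game state Blueprint that starts background music, and in some levels a media source, when play begins, based on the current level name.
; On ThirdPersonMap it adds an audio component flagged as UI sound, plays the level track and stores the component in MusicAudioComponent.
; On any other level it opens a media source on the Media player and randomly plays one of two 2D tracks, SHADOWBORN or DARK_ARIA.
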(event EventBeginPlay
  (bind _returnvalue (Game|GetCurrentLevelName true))
  (if (Utilities|Enum|Equal(Enum) _returnvalue "ThirdPersonMap")
    (bind _returnvalue_2 (AddComponent|AddAudioComponent false))
    (Class|AudioComponent|SetUISound _returnvalue_2 true)
    (Audio|Components|Audio|SetSound _returnvalue_2 "/Game/Audio/LEveL.LEveL")
    (Audio|Components|Audio|Play _returnvalue_2 0.0)
    (Variables|Default|SetMusicAudioComponent _returnvalue_2)
    (else
      (Media|MediaPlayer|OpenSource (Variables|Default|GetMedia) "/Game/UIs/0212.0212")
      (if (Math|Random|RandomBool)
        (Audio|PlaySound2D "/Game/Audio/SHADOWBORN.SHADOWBORN" 1.0 1.0 0.0 0 0)
        (else
          (Audio|PlaySound2D "/Game/Audio/DARK_ARIA.DARK_ARIA" 1.0 1.0 0.0 0 0))))))

(event EventTick
  (params (DeltaSeconds :type Float%20%28single-precision%29)))

(fn ConstructionScript)